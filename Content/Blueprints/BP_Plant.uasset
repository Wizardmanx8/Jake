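; BP_Plant is a plant actor that can grow by spawning another copy of itself while the player is near.
; Its GrowthTrigger overlap toggles CanGrow and the ThirdPersonCharacter's CanInteract flag.
; PlantGrow, when CanGrow is set, spawns a BP_Plant at component W's location unless colliding, then stores the new plant's W transform in NextSpawnPoint.
; AddPlant duplicates that spawn logic without the check.
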(event `self.GrowthTrigger.OnComponentBeginOverlap`
  (params (OverlappedComponent :type "PrimitiveComponent Object Reference") (OtherActor :type "Actor Object Reference") (OtherComp :type "PrimitiveComponent Object Reference") (OtherBodyIndex :type Integer) (bFromSweep :type Boolean) (SweepResult :type "HitResult Structure (by ref)"))
  (bind _asthird_person_character (cast `/Game/Blueprints/ThirdPersonCharacter` OtherActor))
  (set `/Game/Blueprints/ThirdPersonCharacter.CanInteract` true _asthird_person_character)
  (set `self.CanGrow` true))

(event `self.GrowthTrigger.OnComponentEndOverlap`
  (params (OverlappedComponent :type "PrimitiveComponent Object Reference") (OtherActor :type "Actor Object Reference") (OtherComp :type "PrimitiveComponent Object Reference") (OtherBodyIndex :type Integer))
  (bind _asthird_person_character (cast `/Game/Blueprints/ThirdPersonCharacter` OtherActor))
  (set `/Game/Blueprints/ThirdPersonCharacter.CanInteract` false _asthird_person_character)
  (set `self.CanGrow` false))

(event `Plant Grow`
  ;[1 1 1] Adds 1 plant and sets it to become the beginnig of another plant
  (if (`self.CanGrow`)
    (bind _returnvalue (`|SpawnActorFromClass` "BP_Plant_C" (`KismetMathLibrary.Conv_VectorToTransform` (`SceneComponent.K2_GetComponentLocation` (`self.w`))) "DontSpawnIfColliding" "OverrideRootScale" null null))
    (bind _plantendtransform (`self.LocateNextPlant` _returnvalue))
    (set `self.NextSpawnPoint` _plantendtransform)))

(fn `AddPlant`
  ;[1 1 1] Adds 1 plant and sets it to become the beginnig of another plant
  (bind _returnvalue (`|SpawnActorFromClass` "BP_Plant_C" (`KismetMathLibrary.Conv_VectorToTransform` (`SceneComponent.K2_GetComponentLocation` (`self.w`))) "DontSpawnIfColliding" "OverrideRootScale" null null))
  (bind _plantendtransform (`self.LocateNextPlant` _returnvalue))
  (set `self.NextSpawnPoint` _plantendtransform))

(fn `LocateNextPlant`
  (returns (PlantEndTransform :type "Transform Structure"))
  (return (`SceneComponent.K2_GetComponentToWorld` (`self.w`))))

(fn `UserConstructionScript`)